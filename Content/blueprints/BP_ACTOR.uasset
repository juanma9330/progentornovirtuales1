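; BP_ACTOR is a simple actor that reports its stats and moves and spins continuously.
; On BeginPlay it prints its name, health and defense (Nombre, Vida, Defensa) on screen in a configurable color.
; Each Tick adds Velocidad as a world offset without sweep and VelocidadRotación as a world rotation, neither scaled by delta time, so motion depends on frame rate.
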(event EventBeginPlay
  (Development|PrintString (Utilities|String|Append "Nombre: 
 " (Variables|Propiedades|GetNombre) " 
Vida:" (Utilities|String|ToString(Integer) (Variables|Propiedades|GetVida)) " 
Defensa;" (Utilities|String|ToString(Float) (Variables|Propiedades|GetDefensa))) true true (Variables|Propiedades|GetColor%20Mensaje) 3e+01))

(event EventTick
  (params (DeltaSeconds :type Float%20%28single-precision%29))
  (Transformation|AddActorWorldOffset (Variables|Propiedades|GetVelocidad))
  (Class|Actor|AddActorWorldRotation (Variables|Propiedades|GetVelocidadRotación)))

(fn ConstructionScript)